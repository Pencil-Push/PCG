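; WheelBP is an actor that spins like a wheel when the player presses F, then slows to a stop.
; It enables input for player 0 on BeginPlay, and F sets a random starting speed and a rotation flag.
; Tick lowers that speed at a constant rate and applies it as local yaw until it reaches zero.
; The yaw step is per frame, so spin distance depends on frame rate.
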(event EventBeginPlay
  (Input|EnableInput (Game|GetPlayerController 0)))

(event EventTick
  (params (DeltaSeconds :type Float%20%28single-precision%29))
  (Variables|Default|SetDelta%20Seconds DeltaSeconds)
  (if (Variables|Default|GetRotation)
    (bind _output_get (Variables|Default|SetRandom%20Rotation (- (Variables|Default|GetRandom%20Rotation) (* (Variables|Default|GetDelta%20Seconds) (Math|Random|RandomFloatinRange 0.5 0.5)))))
    (if (> _output_get 0.0)
      (Transformation|AddActorLocalRotation (Math|Rotator|MakeRotator 0.0 0.0 _output_get) false false)
      (else
        (Variables|Default|SetRotation false)))))

(event Input|KeyboardEvents|F
  (params (Key :type Key%20Structure :default "None"))
  (:Pressed
    (Variables|Default|SetRotation true)
    (Variables|Default|SetRandom%20Rotation (Math|Random|RandomFloatinRange 5.0 1e+01))))

(fn ConstructionScript)